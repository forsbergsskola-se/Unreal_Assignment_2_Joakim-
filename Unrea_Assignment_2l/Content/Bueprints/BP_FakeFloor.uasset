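; BP_FakeFloor is a trap floor tile that disappears shortly after something overlaps its trigger box.
; The overlap waits a second, destroys the owning actor, then attempts to spawn a replacement at the tile transform after another delay.
; That respawn is scheduled on the actor just destroyed, so it is unlikely to run.
; Both branch conditions are hardcoded true, and the player-character cast is disconnected, leaving the trigger unfiltered.
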(event OnComponentBeginOverlap(Box)
  (params (OverlappedComponent :type Primitive%20Component%20Object%20Reference) (OtherActor :type Actor%20Object%20Reference) (OtherComp :type Primitive%20Component%20Object%20Reference) (OtherBodyIndex :type Integer) (bFromSweep :type Boolean) (SweepResult :type Hit%20Result%20Structure%20%28by%20ref%29))
  (if true
    (Utilities|FlowControl|Delay 1.0)
    (Actor|DestroyActor (Components|GetOwner (Variables|Default|GetCube)))
    (if true
      (Utilities|FlowControl|Delay 1.0)
      (Game|SpawnActorfromClass "BP_FakeFloor_C" (Class|TileMapBlueprintLibrary|GetTileTransform) "AlwaysSpawn" 0 0)
      (else
        (Development|PrintString "NOT AVAIBLE TO RESPAWN FAKE FLOOR")))
    (else
      (Development|PrintString "Wrong READING"))))

(event EventBeginPlay)

(event Collision|EventActorBeginOverlap
  (params (OtherActor :type Actor%20Object%20Reference)))

(event EventTick
  (params (DeltaSeconds :type Float%20%28single-precision%29)))

(fn ConstructionScript)
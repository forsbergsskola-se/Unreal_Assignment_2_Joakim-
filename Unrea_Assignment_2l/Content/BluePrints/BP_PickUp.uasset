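; BP_PickUp is a super jump power-up that temporarily raises the player character's jump velocity.
; Any actor overlap removes its sphere and collision components, boosts player 0's jump, then restores a fixed value after a delay.
; It then spawns a fresh copy at its root transform to respawn, without destroying the original actor.
; Tick rotates the pickup and plays a timeline that applies local movement offsets.
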(event Collision|EventActorBeginOverlap
  (params (OtherActor :type Actor%20Object%20Reference))
  (bind _returnvalue (Game|GetPlayerCharacter 0))
  (bind _charactermovement (Variables|/Script/Engine.Character|GetCharacterMovement _returnvalue))
  (Components|DestroyComponent (Variables|Default|GetSphere))
  (Components|DestroyComponent (Variables|Default|GetCollision))
  (Development|PrintString "Super Jump Is Active")
  (Variables|/Script/Engine.CharacterMovementComponent|SetJumpZVelocity _charactermovement 1.6e+03)
  (Utilities|FlowControl|Delay 1e+01)
  (Variables|/Script/Engine.CharacterMovementComponent|SetJumpZVelocity _charactermovement 7e+02)
  (Development|PrintString "Super Jump Is Deactivated")
  (Game|SpawnActorfromClass "BP_PickUp_C" (Transformation|GetWorldTransform (Variables|Default|GetDefaultSceneRoot)) "AlwaysSpawn" 0 0))

(event EventTick
  (params (DeltaSeconds :type Float%20%28single-precision%29))
  (Transformation|AddActorLocalRotation "0,1.000000, 0" false false)
  (bind _newtrack_0 (Timeline|Timeline_0 Play)
    (:Update
      (Transformation|AddActorLocalOffset _newtrack_0 false false))))

(fn ConstructionScript)